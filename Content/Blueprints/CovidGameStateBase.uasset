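; CovidGameStateBase is the game state of an epidemic game, tracking population, infected, isolated and dead counts.
; AllSetState seeds the counts and isolation capacity (Insolution), and add/remove functions adjust them, with new isolations limited by that capacity.
; RemoveInfected calls ResultEvent on CovidGameModeBase when no infected remain and deaths differ from the population.
; AddDead calls FailedEvent there once deaths reach the population.
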(event EventBeginPlay)

(event EventTick
  (params (DeltaSeconds :type Float%20%28single-precision%29)))

(fn ConstructionScript)

(fn AllSetState
  (params (InfectedInput :type Integer) (InsolutionInput :type Integer) (IsolutorInput :type Integer) (PopulationInput :type Integer))
  (Variables|Default|SetInfected InfectedInput)
  (Variables|Default|SetInsolution InsolutionInput)
  (Variables|Default|SetIsolutor IsolutorInput)
  (Variables|Default|SetPopulation PopulationInput))

(fn AddInfected
  (Math|Integer|IncrementInt (Variables|Default|GetInfected)))

(fn RemoveInfected
  (bind _infected (Variables|Default|GetInfected))
  (Math|Integer|DecrementInt _infected
    (:%20%20
      (bind _ascovid_game_mode_base (Utilities|Casting|CastToCovidGameModeBase (Game|GetGameMode)))
      (if (and (!= (Variables|Default|GetDead) (Variables|Default|GetPopulation)) (<= _infected 0))
        (Default|ResultEvent _ascovid_game_mode_base)))))

(fn AddIsolutor
  (if (< (Variables|Default|GetIsolutor) (Variables|Default|GetInsolution))
    (Variables|Default|SetIsolutor (+ (Variables|Default|GetIsolutor) 1))))

(fn RemoveIsolutor
  (Math|Integer|DecrementInt (Variables|Default|GetIsolutor)))

(fn IsolutorAble
  (return (< (Variables|Default|GetIsolutor) (Variables|Default|GetInsolution))))

(fn AddDead
  (bind _ascovid_game_mode_base (Utilities|Casting|CastToCovidGameModeBase (Game|GetGameMode)))
  (bind _result (Math|Integer|IncrementInt (Variables|Default|GetDead))
    (:%20%20
      (if (>= _result (Variables|Default|GetPopulation))
        (Default|FailedEvent _ascovid_game_mode_base)))))