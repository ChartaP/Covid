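; Player controller for a COVID-themed game that routes player input to the CovidPlayerChar it caches on BeginPlay.
; View axes drive yaw and pitch, while movement axes move the character along the control rotation's forward and right vectors.
; Number keys switch between two weapons, and Fire starts a temperature check or gives a mask depending on the active one.
; Arrest calls TargetArrest with a running counter that increments on each press.
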(event EventBeginPlay
  (bind _ascovid_player_char (Utilities|Casting|CastToCovidPlayerChar (Game|GetPlayerCharacter 0)))
  (Variables|Default|SetMyPlayerChar _ascovid_player_char))

(event EventTick
  (params (DeltaSeconds :type Float%20%28single-precision%29)))

(event Input|ActionEvents|InputActionNum1
  (params (Key :type Key%20Structure :default "None"))
  (:Pressed
    (Default|WeaponChange (Variables|Default|GetMyPlayerChar) 1)))

(event Input|ActionEvents|InputActionNum2
  (params (Key :type Key%20Structure :default "None"))
  (:Pressed
    (Default|WeaponChange (Variables|Default|GetMyPlayerChar) 2)))

(event Input|ActionEvents|InputActionFire
  (params (Key :type Key%20Structure :default "None"))
  (bind _myplayerchar (Variables|Default|GetMyPlayerChar))
  (:Pressed
    (switch int (Variables|/Game/Blueprints/CovidPlayerChar.CovidPlayerChar_C|GetWeapon _myplayerchar)
      (:1
        (Default|TempCheckStart _myplayerchar))
      (:2
        (Default|GiveMask _myplayerchar)))))

(event Input|ActionEvents|InputActionArrest
  (params (Key :type Key%20Structure :default "None"))
  (bind _numbering (Variables|Default|GetNumbering))
  (:Pressed
    (Default|TargetArrest (Variables|Default|GetMyPlayerChar) _numbering)
    (Math|Integer|IncrementInt _numbering)))

(event Input|AxisEvents|InputAxisViewH
  (params (AxisValue :type Float%20%28single-precision%29))
  (Pawn|Input|AddControllerYawInput (Variables|Default|GetMyPlayerChar) AxisValue))

(event Input|AxisEvents|InputAxisViewV
  (params (AxisValue :type Float%20%28single-precision%29))
  (Pawn|Input|AddControllerPitchInput (Variables|Default|GetMyPlayerChar) AxisValue))

(event Input|AxisEvents|InputAxisMoveForward
  (params (AxisValue :type Float%20%28single-precision%29))
  (bind _myplayerchar (Variables|Default|GetMyPlayerChar))
  (Pawn|Input|AddMovementInput _myplayerchar (Math|Vector|GetForwardVector (Pawn|GetControlRotation _myplayerchar :!class /Script/Engine.Pawn)) AxisValue false))

(event Input|AxisEvents|InputAxisMoveRight
  (params (AxisValue :type Float%20%28single-precision%29))
  (bind _myplayerchar (Variables|Default|GetMyPlayerChar))
  (Pawn|Input|AddMovementInput _myplayerchar (Math|Vector|GetRightVector (Pawn|GetControlRotation _myplayerchar :!class /Script/Engine.Pawn)) AxisValue false))

(fn ConstructionScript)