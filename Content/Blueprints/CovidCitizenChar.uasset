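; Citizen character for a COVID quarantine game, randomly given a mask, infection and matching body temperature range at spawn.
; StartIsolutor teleports it below the map and runs a timed CheckCovid that posts a Korean test-result headline to CovidGameStateBase.
; Positives get a timed treatment before EndIsolutor cures them and returns them to a random spot; negatives return immediately.
; Infected and isolated counts go to the game state, and Tick drives the walk animation outside isolation.
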(event EventBeginPlay
  (CallFunction|TakeMask (Math|Random|RandomBoolwithWeight 0.5))
  (bind _takeresult (CallFunction|TakeCovid (Math|Random|RandomBoolwithWeight 0.2)))
  (if _takeresult
    (bind _ascovid_game_state_base (Utilities|Casting|CastToCovidGameStateBase (Game|GetGameState)))
    (Default|AddInfected _ascovid_game_state_base)))

(event Collision|EventActorBeginOverlap
  (params (OtherActor :type Actor%20Object%20Reference)))

(event EventTick
  (params (DeltaSeconds :type Float%20%28single-precision%29))
  (if (not (Variables|Default|GetIsIsolutor))
    (CallFunction|AnimUpdate)))

(fn ConstructionScript)

(fn TakeMask
  (params (IsTake :type Boolean))
  (bind _output_get (Variables|Default|SetIsMasked IsTake))
  (Rendering|SetVisibility (Variables|Default|GetMask) _output_get false)
  (return _output_get))

(fn TakeCovid
  (params (IsCovid :type Boolean))
  (bind _output_get (Variables|Default|SetIsCovid IsCovid))
  (if _output_get
    (Variables|Default|SetTemp (Math|Random|RandomFloatinRange 37.0 4e+01))
    (else
      (Variables|Default|SetTemp (Math|Random|RandomFloatinRange 35.0 38.0))))
  (return _output_get))

(fn AnimUpdate
  (bind _charactermovement (Variables|Character|GetCharacterMovement))
  (bind _returnvalue (Pawn|Components|CharacterMovement|GetLastUpdateVelocity _charactermovement))
  (bind _returnvalue_2 (Math|Vector|VectorLength _returnvalue))
  (bind _aslp_skeleton_anim (Utilities|Casting|CastTolpSkeleton_Anim (Components|SkeletalMesh|GetAnimInstance (Variables|Character|GetMesh))))
  (Variables|/Game/FreeAsset/Model/lpSkeleton_Anim.lpSkeleton_Anim_C|SetIsWalk _aslp_skeleton_anim (not (and (< _returnvalue_2 1.0) (> _returnvalue_2 -1.0)))))

(fn StartIsolutor
  (params (Numbering :type Integer))
  (bind _ascovid_game_state_base (Utilities|Casting|CastToCovidGameStateBase (Game|GetGameState)))
  (Variables|Default|SetNumer Numbering)
  (Default|AddIsolutor _ascovid_game_state_base)
  (Variables|Default|SetIsIsolutor true)
  (Transformation|SetActorLocation "0, 0,-4000.000000" false true)
  (Utilities|Time|SetTimerbyFunctionName 0 "CheckCovid" 1e+01))

(fn EndIsolutor
  (bind _ascovid_game_state_base (Utilities|Casting|CastToCovidGameStateBase (Game|GetGameState)))
  (if (Variables|Default|GetIsCovid)
    (Variables|Default|SetIsCovid false)
    (Default|RemoveInfected _ascovid_game_state_base))
  (Variables|Default|SetIsIsolutor false)
  (Default|RemoveIsolutor _ascovid_game_state_base)
  (Transformation|SetActorLocation (Math|Vector|MakeVector (Math|Random|RandomFloatinRange -2e+03 2e+03) (Math|Random|RandomFloatinRange -2e+03 2e+03) 1e+02) false true))

(fn CheckCovid
  (bind _ascovid_game_state_base (Utilities|Casting|CastToCovidGameStateBase (Game|GetGameState)))
  (if (Variables|Default|GetIsCovid)
    (Variables|/Game/Blueprints/CovidGameStateBase.CovidGameStateBase_C|SetNewsText _ascovid_game_state_base (Utilities|Text|ToText(String) (Utilities|String|Append (Utilities|String|ToString(Integer) (Variables|Default|GetNumer)) "번 격리자는 양성판정으로 치료에 들어갑니다")))
    (Utilities|Time|SetTimerbyFunctionName 0 "EndIsolutor" 1e+01)
    (else
      (Variables|/Game/Blueprints/CovidGameStateBase.CovidGameStateBase_C|SetNewsText _ascovid_game_state_base (Utilities|Text|ToText(String) (Utilities|String|Append (Utilities|String|ToString(Integer) (Variables|Default|GetNumer)) "번 격리자는 음성판정 받았습니다")))
      (CallFunction|EndIsolutor))))