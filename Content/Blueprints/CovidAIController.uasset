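; AI controller that makes a CovidCitizenChar pawn wander randomly around the level.
; On BeginPlay it caches the controlled citizen and starts a looping ChangeDir timer, with its interval randomized once between a few seconds.
; ChangeDir moves the citizen to a random nearby XY offset without pathfinding.
; Tick reruns the same setup whenever the cached citizen reference is invalid.
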(event EventBeginPlay
  (bind _ascovid_citizen_char (Utilities|Casting|CastToCovidCitizenChar (Pawn|GetControlledPawn)))
  (Variables|Default|SetMyCitizenChar _ascovid_citizen_char)
  (CallFunction|ChangeDir)
  (Utilities|Time|SetTimerbyFunctionName 0 "ChangeDir" (Math|Random|RandomFloatinRange 3.0 5.0) true))

(event EventTick
  (params (DeltaSeconds :type Float%20%28single-precision%29))
  (if (not (Utilities|IsValid (Variables|Default|GetMyCitizenChar)))
    (bind _ascovid_citizen_char (Utilities|Casting|CastToCovidCitizenChar (Pawn|GetControlledPawn)))
    (Variables|Default|SetMyCitizenChar _ascovid_citizen_char)
    (CallFunction|ChangeDir)
    (Utilities|Time|SetTimerbyFunctionName 0 "ChangeDir" (Math|Random|RandomFloatinRange 3.0 5.0) true)))

(fn ConstructionScript)

(fn ChangeDir
  (AI|Navigation|MovetoLocation (+ (Transformation|GetActorLocation (Variables|Default|GetMyCitizenChar)) (Math|Vector|MakeVector (Math|Random|RandomFloatinRange -5e+02 5e+02) (Math|Random|RandomFloatinRange -5e+02 5e+02) 0.0)) -1.0 true false false true 0))