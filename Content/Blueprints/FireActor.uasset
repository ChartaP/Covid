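; FireActor is a short-lived fire projectile that kills and burns CovidCitizenChar characters it touches.
; Fire sets its travel direction, and Tick moves it along that vector at a fixed speed without sweeping.
; Overlapping a citizen with the Col component calls Dead and IsBurn on it, then Out destroys the projectile.
; A timer started on BeginPlay also calls Out, so the projectile expires in under a second.
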(event OnComponentBeginOverlap(Col)
  (params (OverlappedComponent :type Primitive%20Component%20Object%20Reference) (OtherActor :type Actor%20Object%20Reference) (OtherComp :type Primitive%20Component%20Object%20Reference) (OtherBodyIndex :type Integer) (bFromSweep :type Boolean) (SweepResult :type Hit%20Result%20Structure%20%28by%20ref%29))
  (bind _ascovid_citizen_char (Utilities|Casting|CastToCovidCitizenChar OtherActor))
  (Default|Dead _ascovid_citizen_char)
  (Default|IsBurn _ascovid_citizen_char)
  (CallFunction|Out))

(event EventBeginPlay
  (Utilities|Time|SetTimerbyFunctionName 0 "Out" 0.8))

(event Collision|EventActorBeginOverlap
  (params (OtherActor :type Actor%20Object%20Reference)))

(event EventTick
  (params (DeltaSeconds :type Float%20%28single-precision%29))
  (Transformation|SetActorLocation (+ (Transformation|GetActorLocation) (* (Variables|Default|GetDirection) (* DeltaSeconds 1.2e+03))) false false))

(fn ConstructionScript)

(fn Fire
  (params (DirectionInput :type Vector))
  (Variables|Default|SetDirection DirectionInput))

(fn Out
  (Utilities|Time|ClearTimerbyFunctionName 0 "Out")
  (Actor|DestroyActor))