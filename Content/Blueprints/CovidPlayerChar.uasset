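; Player character for a COVID screening game, able to hand masks to citizens and check their temperature.
; BeginPlay adds the HUD, and a box overlap sets or clears the target CovidCitizenChar while printing debug info.
; WeaponChange toggles thermometer and mask visibility.
; Temperature checks run on a looping function-name timer that advances progress, sets Korean result or failure messages, then clears them; TargetArrest is an empty stub.
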(event OnComponentBeginOverlap(BoxCol)
  (params (OverlappedComponent :type Primitive%20Component%20Object%20Reference) (OtherActor :type Actor%20Object%20Reference) (OtherComp :type Primitive%20Component%20Object%20Reference) (OtherBodyIndex :type Integer) (bFromSweep :type Boolean) (SweepResult :type Hit%20Result%20Structure%20%28by%20ref%29))
  (bind _ascovid_citizen_char (Utilities|Casting|CastToCovidCitizenChar OtherActor))
  (Variables|Character|SetTarget _ascovid_citizen_char)
  (Development|PrintString "BoxColStart")
  (Development|PrintString (Utilities|String|Append "IsCovid : " (Utilities|String|ToString(Boolean) (Variables|/Game/Blueprints/CovidCitizenChar.CovidCitizenChar_C|GetIsCovid (Variables|Character|GetTarget)))))
  (Development|PrintString (Utilities|String|Append "IsMasked : " (Utilities|String|ToString(Boolean) (Variables|/Game/Blueprints/CovidCitizenChar.CovidCitizenChar_C|GetIsMasked (Variables|Character|GetTarget)))))
  (Development|PrintString (Utilities|String|Append "Temp : " (Utilities|String|ToString(Float) (Variables|/Game/Blueprints/CovidCitizenChar.CovidCitizenChar_C|GetTemp (Variables|Character|GetTarget))))))

(event OnComponentEndOverlap(BoxCol)
  (params (OverlappedComponent :type Primitive%20Component%20Object%20Reference) (OtherActor :type Actor%20Object%20Reference) (OtherComp :type Primitive%20Component%20Object%20Reference) (OtherBodyIndex :type Integer))
  (Development|PrintString "BoxColEnd")
  (if (== OtherActor (Variables|Character|GetTarget))
    (Variables|Character|SetTarget 0)))

(event EventBeginPlay
  (bind _returnvalue (UserInterface|CreateWidget "/Game/Blueprints/CovidHUD.CovidHUD_C"))
  (UserInterface|Viewport|AddtoViewport _returnvalue 0))

(event Collision|EventActorBeginOverlap
  (params (OtherActor :type Actor%20Object%20Reference)))

(event EventTick
  (params (DeltaSeconds :type Float%20%28single-precision%29)))

(fn ConstructionScript)

(fn WeaponChange
  (params (WeaponNum :type Integer))
  (bind _mask (Variables|Default|GetMask))
  (bind _therometer (Variables|Default|GetTherometer))
  (bind _output_get (Variables|Default|SetWeapon WeaponNum))
  (switch int _output_get
    (:1
      (Rendering|SetVisibility _mask false false)
      (Rendering|SetVisibility _therometer true false))
    (:2
      (Rendering|SetVisibility _mask true false)
      (Rendering|SetVisibility _therometer false false))))

(fn GiveMask
  (bind _target (Variables|Character|GetTarget))
  (if (Utilities|IsValid _target)
    (Default|TakeMask _target)))

(fn TargetArrest)

(fn TempCheckStart
  (if (Utilities|IsValid (Variables|Character|GetTarget))
    (Variables|Default|SetIsTemp true)
    (Variables|Default|SetPercent 0.0)
    (Utilities|Time|SetTimerbyFunctionName 0 "TempChecking" 0.01 true)
    (else
      (Variables|Default|SetUpMsg "대상이 없습니다")
      (Utilities|Time|SetTimerbyFunctionName 0 "ClearMsg" 2.0))))

(fn TempChecking
  (bind _target (Variables|Character|GetTarget))
  (if (Utilities|IsValid _target)
    (Variables|Default|SetUpMsg "체온측정 중...")
    (Variables|Default|SetPercent (+ (Variables|Default|GetPercent) 0.01))
    (if (>= (Variables|Default|GetPercent) 1.0)
      (Variables|Default|SetUpMsg (Utilities|Text|ToText(String) (Utilities|String|Append "체온 : " (Utilities|String|ToString(Float) (Variables|/Game/Blueprints/CovidCitizenChar.CovidCitizenChar_C|GetTemp _target)))))
      (if (Variables|/Game/Blueprints/CovidCitizenChar.CovidCitizenChar_C|GetIsCovid _target)
        (Variables|Default|SetDownMsg "유증상자")
        (else
          (Variables|Default|SetDownMsg "정상 체온")))
      (Class|KismetSystemLibrary|PauseTimer 0 "TempChecking" :!label _label)
      (Variables|Default|SetIsTemp false)
      (Utilities|Time|SetTimerbyFunctionName 0 "ClearMsg" 2.0))
    (else
      (Variables|Default|SetUpMsg "측정실패")
      (goto _label))))

(fn ClearMsg
  (Variables|Default|SetUpMsg "")
  (Variables|Default|SetDownMsg ""))